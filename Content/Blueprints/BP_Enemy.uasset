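; BP_Enemy is an enemy pawn that wanders at random, chases pawns it sees and deals damage on contact.
; From BeginPlay it moves to random navigable points near itself, pausing briefly after each success or failure before picking the next.
; PawnSensing sightings start a move toward the seen pawn, with no explicit stop of the wander loop.
; Capsule hits apply damage to whatever actor is struck, without filtering.
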(event OnSeePawn(PawnSensing)
  (params (Pawn :type Pawn%20Object%20Reference))
  (AI|AIMoveTo self "0, 0, 0" Pawn 5.0 false))

(event OnComponentHit(CapsuleComponent)
  (params (HitComponent :type Primitive%20Component%20Object%20Reference) (OtherActor :type Actor%20Object%20Reference) (OtherComp :type Primitive%20Component%20Object%20Reference) (NormalImpulse :type Vector :default "0, 0, 0") (Hit :type Hit%20Result%20Structure%20%28by%20ref%29))
  (Game|Damage|ApplyDamage OtherActor 1.0 0 0))

(event Custom|MoveToRandomLocation
  (bind _randomlocation (Class|NavigationSystemV1|GetRandomLocationinNavigableRadius (Transformation|GetActorLocation) 5e+02 0 0))
  (AI|AIMoveTo self _randomlocation 0 5.0 false
    (:OnSuccess
      _)
    (:OnFail
      _))
  (Utilities|FlowControl|Delay (Math|Random|RandomFloatinRange 0.5 3.0))
  (CallFunction|MovetoRandomLocation))

(event EventBeginPlay
  (CallFunction|MovetoRandomLocation))

(fn ConstructionScript)