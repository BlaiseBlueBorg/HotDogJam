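; Actor that records the third-person character's movement from BeginPlay and replays it when Enter is pressed, quitting the game when the replay ends.
; A self-calling Delay timer stores timestamped location and rotation samples, only when location changes.
; Enter stops recording, disables character input, teleports it to InitLocation and restarts the clock.
; Playback applies at most one due sample per timer step, using swept location moves.
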(event Custom|TimerEvent
  (bind _timervalue (Variables|General|GetTimerValue))
  ;[1 0.1365 0.1365] Timer
  (CallFunction|RecordTransform)
  (if (Variables|General|GetTimerActivated)
    (Utilities|FlowControl|Delay _timervalue)
    (bind _output_get (Variables|General|SetCurrentTime (+ _timervalue (Variables|General|GetCurrentTime))))
    ;;[1 1 1] VisibleTimer
    (Development|PrintString (Utilities|String|ToString(Float) _output_get) true true "(R=0.000000,G=0.660000,B=1.000000,A=1.000000)" (Variables|General|GetTimerValue))
    (CallFunction|TimerEvent)))

(event Custom|PlaybackTimer
  (bind _timervalue (Variables|General|GetTimerValue))
  ;[1 0.2253 0.4205] PlaybackSpaceTimer
  (Utilities|FlowControl|Delay _timervalue)
  (bind _output_get (Variables|General|SetCurrentTime (+ _timervalue (Variables|General|GetCurrentTime))))
  (Development|PrintString (Utilities|String|ToString(Float) _output_get) true true "(R=0.000000,G=0.660000,B=1.000000,A=1.000000)" _timervalue)
  (if (< 0 (Utilities|Array|Length (Variables|Transform|GetTransformStructList)))
    (CallFunction|CheckTransformList)
    (bind _output_get_2 (Variables|General|SetTimerOver (>= (Variables|General|GetCurrentTime) (Variables|General|GetTimerEnd))))
    (if _output_get_2
      (Development|PrintString "REPLAY OVER")
      (Game|QuitGame 0 "Quit" false)
      (else
        (CallFunction|PlaybackTimer)))))

(event EventBeginPlay
  ;[0.07301 0.3949 1] Get Player Pawn
  (Input|EnableInput (Game|GetPlayerController 0))
  (bind _outactors (Actor|GetAllActorsOfClass "/Game/ThirdPerson/Blueprints/BP_ThirdPersonCharacter.BP_ThirdPersonCharacter_C"))
  (Variables|General|SetCharacterPawn (Utilities|Array|Get(acopy) _outactors))
  ;[1 0 0] Start Timer
  (Variables|General|SetTimerActivated true)
  (CallFunction|TimerEvent))

(event Input|KeyboardEvents|Enter
  (params (Key :type Key%20Structure :default "None"))
  ;[0.4956 0.4698 1] Playback
  (:Pressed
    (Development|PrintString "Timer Stopped")
    (Input|DisableInput (Variables|General|GetCharacterPawn) (Game|GetPlayerController 0))
    (Variables|General|SetTimerActivated false)
    (bind _output_get (Variables|General|SetTimerEnd (Variables|General|GetCurrentTime)))
    (Variables|General|SetCurrentTime 0.0)
    (Transformation|SetActorLocation (Variables|General|GetCharacterPawn) (Variables|Transform|GetInitLocation) false true)
    (CallFunction|PlaybackTimer)))

(fn ConstructionScript)

(fn CheckTransformList
  (bind _transformstructlist (Variables|Transform|GetTransformStructList))
  (bind _transformlistposition (Variables|Transform|GetTransformListPosition))
  (bind _characterpawn (Variables|General|GetCharacterPawn))
  (bind _output (Utilities|Array|Get(acopy) _transformstructlist _transformlistposition))
  (if (>= (Variables|General|GetCurrentTime) (.time _output))
    (Transformation|SetActorLocation _characterpawn (.location _output) true false)
    (Transformation|SetActorRotation _characterpawn (.rotation _output))
    (Math|Integer|IncrementInt (Variables|Transform|GetTransformListPosition)
      (:%20%20
        (return)))))

(fn RecordTransform
  (bind _characterpawn (Variables|General|GetCharacterPawn))
  (bind _returnvalue (Transformation|GetActorTransform _characterpawn))
  (if (Utilities|Operators|EqualEqual (.location _returnvalue) (Variables|Transform|GetLastLocation) 0.0)
    (return)
    (else
      (Development|PrintString "MOVING")
      (bind _output_get (Variables|Transform|SetTransformStruct (Utilities|Struct|MakeTiming_Transform_Struct (Variables|General|GetCurrentTime) (.location _returnvalue) (.rotation _returnvalue))))
      (Utilities|Array|Add (Variables|Transform|GetTransformStructList) _output_get)
      (Variables|Transform|SetLastLocation (.location _returnvalue))
      (return))))