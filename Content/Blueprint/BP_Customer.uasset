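; BP_Customer is an AI customer that chases the player and is destroyed when a hot dog hits it.
; PawnSensing seeing a pawn sets PlayerDetected and calls FollowPlayer, which runs a single AI Move To toward the first player's character.
; Overlap of its box collision with a BP_HotDog destroys the customer; debug strings print on detection and on move completion.
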(event OnComponentBeginOverlap(BoxCollision)
  (params (OverlappedComponent :type Primitive%20Component%20Object%20Reference) (OtherActor :type Actor%20Object%20Reference) (OtherComp :type Primitive%20Component%20Object%20Reference) (OtherBodyIndex :type Integer) (bFromSweep :type Boolean) (SweepResult :type Hit%20Result%20Structure%20%28by%20ref%29))
  ;[1 1 1] Customer Kill
  (Utilities|Casting|CastToBP_HotDog OtherActor)
  (Actor|DestroyActor))

(event OnSeePawn(PawnSensing)
  (params (Pawn :type Pawn%20Object%20Reference))
  (Development|PrintString "seeeeeeeeee youuuu")
  (Variables|Default|SetPlayerDetected? true)
  (CallFunction|FollowPlayer))

(event Custom|FollowPlayer
  (if (Variables|Default|GetPlayerDetected?)
    (AI|AIMoveTo self "0, 0, 0" (Game|GetPlayerCharacter 0) 5.0 false
      (:then
        (Development|PrintString "moved")))))

(event EventBeginPlay)

(fn ConstructionScript)